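; BP_SockSpawner is an actor that periodically spawns and launches socks of random type.
; On BeginPlay it starts a looping two-second timer that calls SpawnSock.
; SpawnSock spawns a BP_Sock at the spawner's transform with one of three randomly chosen SockType values, then applies an impulse to its mesh along the Arrow component's forward vector.
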(event `self.ReceiveBeginPlay`
  (`KismetSystemLibrary.K2_SetTimerDelegate` (delegate `SpawnSock`) 2.0 true))

(event `SpawnSock`
  (bind _returnvalue (`|SpawnActorFromClass` "/Game/Root/Assets/Blueprints/BP_Sock.BP_Sock_C" (`self.GetTransform`) "Undefined" "OverrideRootScale" null (select `int` (`KismetMathLibrary.RandomInteger` 3) :`0` "NewEnumerator0" :`1` "NewEnumerator1" :`2` "NewEnumerator2" :!type "/Game/Root/Core/Player/Blueprints/E_SockTypes Enum") null))
  (`PrimitiveComponent.AddImpulse` (`/Game/Root/Assets/Blueprints/BP_Sock.SM_Sock` _returnvalue) (* (`SceneComponent.GetForwardVector` (`self.Arrow`)) 1000.0) "None" false))

(fn `UserConstructionScript`)