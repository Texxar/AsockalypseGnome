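; Incinerator actor that burns socks to add time through the SockGnome game mode, without adding score.
; A player entering or leaving its Collision volume plays or reverses a timeline that swings the hatch hinge open or closed.
; Socks overlapping the CubeCollision volume are destroyed with a burning sound before the time bonus is granted.
; A calm fire sound plays at its location on BeginPlay.
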(event `self.ReceiveBeginPlay`
  (`GameplayStatics.PlaySoundAtLocation` "/Game/Root/Assets/Audio/SFX/Footsteps/CUE_CalmFire.CUE_CalmFire" (`self.K2_GetActorLocation`) (struct) 1.0 1.0 0.0 null null null)
  (set `self.ClosedRotation` (`SceneComponent.RelativeRotation` (`self.SM_IncineratorHatch`))))

(event `self.Collision.OnComponentBeginOverlap`
  (params (OverlappedComponent :type "PrimitiveComponent Object Reference") (OtherActor :type "Actor Object Reference") (OtherComp :type "PrimitiveComponent Object Reference") (OtherBodyIndex :type Integer) (bFromSweep :type Boolean) (SweepResult :type "HitResult Structure (by ref)"))
  (cast `/Game/Root/Core/Player/Blueprints/Core_PlayerCharacter` OtherActor)
  (set `self.bPlayerInRadius` true)
  (if (not (`self.bHatchIsOpen`))
    (`self.OnOpenHatch`)))

(event `self.Collision.OnComponentEndOverlap`
  (params (OverlappedComponent :type "PrimitiveComponent Object Reference") (OtherActor :type "Actor Object Reference") (OtherComp :type "PrimitiveComponent Object Reference") (OtherBodyIndex :type Integer))
  (cast `/Game/Root/Core/Player/Blueprints/Core_PlayerCharacter` OtherActor)
  (set `self.bPlayerInRadius` false)
  (if (`self.bHatchIsOpen`)
    (`self.OnCloseHatch`)))

(event `OnOpenHatch`
  (bind _closedrotation (`self.ClosedRotation`))
  (set `self.bHatchIsOpen` true)
  (bind (_direction _newtrack_0) (`Timeline|OpenHatchTimeLine` :!label _label)
    (:`Update`
      (`SceneComponent.K2_SetRelativeRotation` (`self.Hinge`) (`KismetMathLibrary.RLerp` _closedrotation (`KismetMathLibrary.ComposeRotators` _closedrotation (struct :`Roll` -180.0)) _newtrack_0) false false))))

(event `OnCloseHatch`
  (set `self.bHatchIsOpen` false)
  (goto _label :!via `Reverse`))

(event `self.CubeCollision.OnComponentBeginOverlap`
  (params (OverlappedComponent :type "PrimitiveComponent Object Reference") (OtherActor :type "Actor Object Reference") (OtherComp :type "PrimitiveComponent Object Reference") (OtherBodyIndex :type Integer) (bFromSweep :type Boolean) (SweepResult :type "HitResult Structure (by ref)"))
  (bind _asbp_sock (cast `/Game/Root/Assets/Blueprints/BP_Sock` OtherActor))
  (`self.K2_DestroyActor` _asbp_sock)
  (`GameplayStatics.PlaySound2D` "/Game/Root/Assets/Audio/SFX/Footsteps/CUE_BurningSock.CUE_BurningSock" 1.0 1.0 0.0 null null)
  (bind _asgm_sock_gnome (cast `/Game/Root/Core/Framework/GM_SockGnome` (`GameplayStatics.GetGameMode`)))
  (`/Game/Root/Core/Framework/GM_SockGnome.AddTime` _asgm_sock_gnome 2 0))

(fn `UserConstructionScript`)