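; BP_OrderBubble is a cloud actor showing a three-sock order that the player fulfils by delivering matching socks.
; The construction script picks each sock mesh by colour, and BeginPlay maps components to colours while timelines grow and wobble the cloud.
; A correct delivery removes one matching sock and adds time and score through GM_SockGnome; a wrong one costs time and plays a sound.
; An empty order fires OrderComplete, then shrinks and destroys the bubble.
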(event `self.ReceiveBeginPlay`
  (`|ExecutionSequence`
    (:`then_0`
      ;[1 1 1] Scale tha actor into existence
      (bind (_direction _alpha) (`Timeline|Timeline_1`)
        (:`Update`
          (`SceneComponent.SetWorldScale3D` (`self.SM_Cloud`) (`KismetMathLibrary.VLerp` (0.0 0.0 0.0) (2.0 2.0 2.0) _alpha)))
        (:`Finished`
          ;[1 1 1] Then start wobble - and loop it
          (`TimelineComponent.SetPlayRate` (`self.Timeline_0`) 3.0)
          (bind (_direction_2 _alpha_2) (`Timeline|Timeline_0`)
            (:`Update`
              (`SceneComponent.SetWorldScale3D` (`self.SM_Cloud`) (* _alpha_2 2.0)))))))
    (:`then_1`
      ;[1 1 1] Make the order of three socks
      (set `self.FullSockOrder` (`|MakeMap` (`self.SM_Sock`) (`self.SockOrder1`) (`self.SM_Sock1`) (`self.SockOrder2`) (`self.SM_Sock2`) (`self.SockOrder3`))))))

(event `OnDeliverSock`
  (params (DeliveredSock :type "/Game/Root/Core/Player/Blueprints/E_SockTypes Enum" :default "NewEnumerator3"))
  (bind _fullsockorder (`self.FullSockOrder`))
  (bind _values (`BlueprintMapLibrary.Map_Values` (`self.FullSockOrder`)))
  (if (`KismetArrayLibrary.Array_Contains` _values DeliveredSock)
    (bind _keys (`BlueprintMapLibrary.Map_Keys` _fullsockorder))
    (for _array_element _keys
      (if (`|EnumEquality` (`BlueprintMapLibrary.Map_Find` _fullsockorder _array_element) DeliveredSock)
        (`BlueprintMapLibrary.Map_Remove` _fullsockorder _array_element)
        (`ActorComponent.K2_DestroyComponent` _array_element)
        (`/Game/Root/Core/Framework/GM_SockGnome.AddTime` (cast `/Game/Root/Core/Framework/GM_SockGnome` (`GameplayStatics.GetGameMode`) :!pure true) 5 1)
        (break)))
    (bind _keys_2 (`BlueprintMapLibrary.Map_Keys` (`self.FullSockOrder`)))
    (if (< (`KismetArrayLibrary.Array_Length` _keys_2) 1)
      (`self.OnOrderComplete`))
    (else
      (`/Game/Root/Core/Framework/GM_SockGnome.AddTime` (cast `/Game/Root/Core/Framework/GM_SockGnome` (`GameplayStatics.GetGameMode`) :!pure true) -5 0)
      (`GameplayStatics.PlaySound2D` (`self.WrongSockSound`) 1.0 1.0 0.0 null null))))

(event `OnOrderComplete`
  (`self.OrderComplete`)
  (`TimelineComponent.SetPlayRate` (`self.Timeline_2`) 3.0)
  (bind (_direction _alpha) (`Timeline|Timeline_2`)
    (:`Update`
      (`SceneComponent.SetWorldScale3D` (`self.SM_Cloud`) (`KismetMathLibrary.VLerp` (2.0 2.0 2.0) (0.0 0.0 0.0) _alpha)))
    (:`Finished`
      (`self.K2_DestroyActor`))))

(fn `UserConstructionScript`
  (for (_array_element _array_index) (`|MakeArray` (`self.SM_Sock`) (`self.SM_Sock1`) (`self.SM_Sock2`))
    (`StaticMeshComponent.SetStaticMesh` _array_element (select `/Game/Root/Core/Player/Blueprints/E_SockTypes` (`|GetArrayItem` (`|MakeArray` (`self.SockOrder1`) (`self.SockOrder2`) (`self.SockOrder3`)) _array_index) :`NewEnumerator3` "/Game/Root/Assets/Meshes/Socks/SM_Sock_01.SM_Sock_01" :`NewEnumerator0` "/Game/Root/Assets/Meshes/Socks/SM_Sock_03.SM_Sock_03" :`NewEnumerator1` "/Game/Root/Assets/Meshes/Socks/SM_Sock_04.SM_Sock_04" :`NewEnumerator2` "/Game/Root/Assets/Meshes/Socks/SM_Sock_02.SM_Sock_02" :!type "StaticMesh Object Reference"))))