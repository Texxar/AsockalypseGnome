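; Sock delivery pipe that takes customer orders, built along a spline with one spline mesh per segment.
; After a random delay it opens its lid and spawns an order bubble of random available sock types, closing and reordering after completion.
; Thrown socks overlapping the pickup are delivered to the active order and replaced by a sock traveling the spline.
; In menu mode it disables pickup and endlessly spawns traveling socks.
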(event `self.ReceiveBeginPlay`
  (if (`self.IsMenuPipe`)
    (`PrimitiveComponent.SetCollisionEnabled` (`self.SockPickup`) "NoCollision")
    (`|SpawnActorFromClass` "/Game/Root/Assets/Blueprints/BP_PipeTravelingSock.BP_PipeTravelingSock_C" (`KismetMathLibrary.MakeTransform` (0.0 0.0 0.0)) "Undefined" "OverrideRootScale" null (`self.Spline`) null :!label _label)
    (`KismetSystemLibrary.Delay` (`KismetMathLibrary.RandomFloatInRange` 0.2 2.0))
    (goto _label)
    (else
      (`|ExecutionSequence`
        (:`then_0`
          (`TimelineComponent.SetPlayRate` (`self.Timeline_1`) 3.0)
          (bind (_direction _newtrack_0) (`Timeline|Timeline_1`)
            (:`Update`
              (`SceneComponent.SetWorldScale3D` (`self.Cone`) _newtrack_0))))
        (:`then_1`
          (`KismetSystemLibrary.Delay` (`KismetMathLibrary.RandomFloatInRange` 0.0 10.0))
          (`self.OnOrderSock`))
        (:`then_2`
          (set `self.GameMode` (cast `/Game/Root/Core/Framework/GM_SockGnome` (`GameplayStatics.GetGameMode`) :!pure true)))))))

(event `self.SockPickup.OnComponentBeginOverlap`
  (params (OverlappedComponent :type "PrimitiveComponent Object Reference") (OtherActor :type "Actor Object Reference") (OtherComp :type "PrimitiveComponent Object Reference") (OtherBodyIndex :type Integer) (bFromSweep :type Boolean) (SweepResult :type "HitResult Structure (by ref)"))
  (bind _asbp_sock (cast `/Game/Root/Assets/Blueprints/BP_Sock` OtherActor))
  (if (`/Game/Root/Assets/Blueprints/BP_Sock.bHasJustBeenThrown` _asbp_sock)
    (`ActorComponent.Activate` (`self.Niagara`) false)
    (bind _orderref (`self.OrderRef`)
      (:`then`
        (`/Game/Root/Assets/Blueprints/BP_OrderBubble.OnDeliverSock` _orderref (`/Game/Root/Assets/Blueprints/BP_Sock.SockType` _asbp_sock))
        (`self.K2_DestroyActor` _asbp_sock)
        (`|SpawnActorFromClass` "/Game/Root/Assets/Blueprints/BP_PipeTravelingSock.BP_PipeTravelingSock_C" (`KismetMathLibrary.MakeTransform` (0.0 0.0 0.0)) "Undefined" "OverrideRootScale" null (`self.Spline`) null))
      (:`else`))))

(event `OnOrderSock`
  (bind (_direction _alpha) (`Timeline|TL_OpenLid` :!via `PlayFromStart`)
    (:`Update`
      (`SceneComponent.K2_SetRelativeRotation` (`self.SM_Lid`) (`KismetMathLibrary.RLerp` (struct) (struct :`Roll` -210.0) _alpha) false false))
    (:`Finished`
      (`GameplayStatics.SpawnSoundAtLocation` "/Game/Root/Assets/Audio/SFX/VoiceLines/CUE_SFX_Gibberish.CUE_SFX_Gibberish" (`self.K2_GetActorLocation`) (struct) 1.0 1.0 0.0 null null)
      (`KismetArrayLibrary.Array_Clear` (`self.SocksToOrder`))
      (for _ (range (+ (`KismetMathLibrary.Clamp` (`KismetMathLibrary.RandomInteger` (`/Game/Root/Core/Framework/GM_SockGnome.SockAmountInOrder` (cast `/Game/Root/Core/Framework/GM_SockGnome` (`GameplayStatics.GetGameMode`) :!pure true))) 1 3) 1))
        (bind _newparam (`/Game/Root/Core/Framework/GM_SockGnome.GetRandomAvailableSockType` (`self.GameMode`)))
        (`KismetArrayLibrary.Array_Add` (`self.SocksToOrder`) _newparam))
      (bind _returnvalue (`|SpawnActorFromClass` "/Game/Root/Assets/Blueprints/BP_OrderBubble.BP_OrderBubble_C" (`SceneComponent.K2_GetComponentToWorld` (`self.OrderSpawnTransform`)) "Undefined" "OverrideRootScale" null (`self.SocksToOrder`) null))
      (bind _output_get (set `self.OrderRef` _returnvalue))
      (add `/Game/Root/Assets/Blueprints/BP_OrderBubble.OrderComplete` _output_get (delegate `OnOrderCompleted`)))))

(event `OnOrderCompleted`
  (bind (_direction _alpha) (`Timeline|Timeline_0` :!via `PlayFromStart`)
    (:`Update`
      (`SceneComponent.K2_SetRelativeRotation` (`self.SM_Lid`) (`KismetMathLibrary.RLerp` (struct :`Roll` -210.0) (struct) _alpha) false false))
    (:`Finished`
      (`KismetSystemLibrary.Delay` (`KismetMathLibrary.RandomFloatInRange` 2.0 10.0))
      (`self.OnOrderSock`))))

(fn `UserConstructionScript`
  (locals (SplineMeshLength :type "Float (double-precision)" :default 500.0))
  (bind _spline (`self.Spline`))
  (for _index (range (+ (- (`SplineComponent.GetNumberOfSplinePoints` (`self.Spline`)) 2) 1))
    (bind _returnvalue (`AddComponent|NODE_AddSplineMeshComponent-0` :`RelativeTransform` (`KismetMathLibrary.MakeTransform` (`SceneComponent.RelativeLocation` (`self.Spline`)))))
    (bind (_location _tangent) (`SplineComponent.GetLocationAndTangentAtSplinePoint` _spline _index "Local"))
    (bind (_location_2 _tangent_2) (`SplineComponent.GetLocationAndTangentAtSplinePoint` _spline (+ _index 1) "Local"))
    (`SplineMeshComponent.SetStartAndEnd` _returnvalue _location _tangent _location_2 _tangent_2 true)))