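; BP_PipeTravelingSock is an actor, by its name a sock, that travels along a pipe spline and destroys itself at the end.
; A looping timer started on BeginPlay moves and rotates it to match SplineToFollow at the current distance in world space.
; Each tick of the timer advances that distance by a fixed step, so speed depends on the timer rate rather than delta time.
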(event `self.ReceiveBeginPlay`
  (`KismetSystemLibrary.K2_SetTimerDelegate` (delegate `TravelAlongPipe`) 0.01 true))

(event `TravelAlongPipe`
  (bind _splinetofollow (`self.SplineToFollow`))
  (bind _distancetravelled (`self.DistanceTravelled`))
  (`self.K2_SetActorLocationAndRotation` (`SplineComponent.GetLocationAtDistanceAlongSpline` _splinetofollow _distancetravelled "World") (`SplineComponent.GetRotationAtDistanceAlongSpline` _splinetofollow _distancetravelled "World"))
  (bind _output_get (set `self.DistanceTravelled` (+ (`self.DistanceTravelled`) 10.0)))
  (if (> _output_get (`SplineComponent.GetSplineLength` (`self.SplineToFollow`)))
    (`self.K2_DestroyActor`)))

(fn `UserConstructionScript`)