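; BP_Sock is a throwable sock actor that comes in several colour and pattern types.
; The construction script picks the mesh material from SockType and auto-activates a spark particle effect for the Rainbow type.
; OnThrow raises a HasJustBeenThrown flag and clears it after a short delay, while a Hit event triggers a splash particle effect.
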(event `OnThrow`
  (set `self.bHasJustBeenThrown` true)
  (`KismetSystemLibrary.Delay` 5.0)
  (set `self.bHasJustBeenThrown` false))

(event `self.ReceiveHit`
  (params (MyComp :type "PrimitiveComponent Object Reference") (Other :type "Actor Object Reference") (OtherComp :type "PrimitiveComponent Object Reference") (bSelfMoved :type Boolean) (HitLocation :type "Vector Structure") (HitNormal :type "Vector Structure") (NormalImpulse :type "Vector Structure") (Hit :type "HitResult Structure (by ref)"))
  (`ActorComponent.Activate` (`self.P_Splash`) false))

(fn `UserConstructionScript`
  (`PrimitiveComponent.SetMaterial` (`self.SM_Sock`) 0 (select `/Game/Root/Core/Player/Blueprints/E_SockTypes` (`self.SockType`) :`NewEnumerator0` "/Game/Root/Assets/Meshes/Socks/MAT_Socks_Red.MAT_Socks_Red" :`NewEnumerator1` "/Game/Root/Assets/Meshes/Socks/MAT_Socks_Blue.MAT_Socks_Blue" :`NewEnumerator2` "/Game/Root/Assets/Meshes/Socks/MAT_Socks_Green.MAT_Socks_Green" :`NewEnumerator4` "/Game/Root/Assets/Meshes/Socks/MAT_Socks_Cat.MAT_Socks_Cat" :`NewEnumerator5` "/Game/Root/Assets/Meshes/Socks/MAT_Socks_PolkaDots.MAT_Socks_PolkaDots" :`NewEnumerator6` "/Game/Root/Assets/Meshes/Socks/MAT_Socks_TwinPeaks.MAT_Socks_TwinPeaks" :`NewEnumerator7` "/Game/Root/Assets/Meshes/Socks/MAT_Socks_Avocado.MAT_Socks_Avocado" :`NewEnumerator8` "/Game/Root/Assets/Meshes/Socks/MAT_Socks_Black.MAT_Socks_Black" :`NewEnumerator9` "/Game/Root/Assets/Meshes/Socks/MAT_Socks_RainBowJoker.MAT_Socks_RainBowJoker" :!type "MaterialInterface Object Reference"))
  (if (`|EnumEquality` (`self.SockType`) "NewEnumerator9")
    (`ActorComponent.SetAutoActivate` (`self.P_Sparks`) true)))