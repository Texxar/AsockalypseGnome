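; Game mode for SockGnome that runs the countdown timer and keeps the total score.
; A looping one-second timer calls UpdateTime, which decrements and prints the remaining time from a 60-second start.
; Other Blueprints call AddTime to add time and score with a confirmation sound.
; The final ten seconds play countdown cues, and reaching zero plays an out-of-time sound and pauses the timer, with no further game-over logic here.
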(event `self.ReceiveBeginPlay`
  (bind _output_get (set `self.StartTime` 60))
  ;[1 1 1] Start time decrease function ( found to the left)
  (set `self.CurrentTime` _output_get)
  (`KismetSystemLibrary.K2_SetTimer` null "UpdateTime" 1.0 true))

(event `AddTime`
  (params (TimeToAdd :type Integer) (ScoreToAdd :type Integer))
  ;[1 1 1] Event to start from OTHER BPs, adding time to the timer.
  ;[1 1 1] Add Score to Total
  (set `self.TotalScore` (+ ScoreToAdd (`self.TotalScore`)))
  (set `self.CurrentTime` (+ (`self.CurrentTime`) TimeToAdd))
  (`GameplayStatics.SpawnSound2D` "/Game/Root/Assets/Audio/UI/CUE_UI_AddedTime.CUE_UI_AddedTime" 1.0 1.0 0.0 null))

(fn `UpdateTime`
  ;[1 1 1] Decrease Time by 1 sec every sec
  (bind _result (`/Engine/EditorBlueprintResources/StandardMacros.DecrementInt` (`self.CurrentTime`))
    (:`  `
      (bind _output_get (set `self.CurrentTime` _result))
      (`KismetSystemLibrary.PrintString` (`KismetStringLibrary.Conv_IntToString` _output_get))
      (if (< (`self.CurrentTime`) 11)
        (if (> (`self.CurrentTime`) 0)
          ;[1 1 1] Play count-down sound when less than 11  sec left
          (bind _returnvalue (`GameplayStatics.SpawnSound2D` "/Game/Root/Assets/Audio/UI/CUE_UI_Countdown.CUE_UI_Countdown" 1.0 1.0 0.0 null))
          (`AudioComponent.SetBoolParameter` _returnvalue "Under11" true)
          (else
            ;[1 1 1] Play out-of-time sound when timer reaches zero
            (`GameplayStatics.SpawnSound2D` "/Game/Root/Assets/Audio/UI/CUE_UI_OutOfTime.CUE_UI_OutOfTime" 1.0 1.0 0.0 null)
            (`KismetSystemLibrary.K2_PauseTimer` null "UpdateTime")))))))

(fn `UserConstructionScript`)